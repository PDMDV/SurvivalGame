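; Construction site actor that shows a building's blueprint mesh until the required resources are gathered and it gets built.
; Tagged Item actors overlapping a box sized for the target building are counted per resource type and shown in a widget.
; StartConstructing, server-only, enables Tick once resources suffice, advancing progress that an OnRep mirrors to client widgets.
; On completion the server destroys the consumed items, spawns the building and removes itself.
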(event `self.ReceiveBeginPlay`
  (bind _boundbox (`self.BoundBox`))
  (bind _buildingclass (`BuildingDataAsset.BuildingClass` (`self.Building Asset`)))
  (bind _requiredresource (`BuildingDataAsset.RequiredResource` (`self.Building Asset`)))
  (bind _returnvalue (`self.GetBoundBoxLocation` _buildingclass))
  ;[1 1 1] Init
  (`StaticMeshComponent.SetStaticMesh` (`self.Mesh`) (`BuildingDataAsset.BlueprintMesh` (`self.Building Asset`)))
  (bind _returnvalue_2 (`KismetMaterialLibrary.CreateDynamicMaterialInstance` "/Game/Survival/Materials/M_Builging_Blueprint.M_Builging_Blueprint"))
  (set `self.DynamicMaterial` _returnvalue_2)
  (for _index (range (`KismetArrayLibrary.Array_Length` (`MeshComponent.GetMaterials` (`self.Mesh`))))
    ;;[1 1 1] Loop body
    (`PrimitiveComponent.SetMaterial` (`self.Mesh`) _index (`self.DynamicMaterial`)))
  (`self.SetBuildingClass` (`BuildingDataAsset.BuildingClass` (`self.Building Asset`)))
  (bind _aswbp_construtciton (cast `/Game/Survival/Blueprints/Widgets/WBP_Construtciton` (`WidgetComponent.GetWidget` (`self.Widget`))))
  (`/Game/Survival/Blueprints/Widgets/WBP_Construtciton.AddResourceRequirement` _aswbp_construtciton (`BuildingDataAsset.RequiredResource` (`self.Building Asset`)))
  (`BlueprintMapLibrary.Map_Clear` (`self.CollectedResources`))
  (bind _keys (`BlueprintMapLibrary.Map_Keys` _requiredresource))
  (for _array_element _keys
    (`BlueprintMapLibrary.Map_Add` (`self.CollectedResources`) _array_element (make `/Game/Survival/Blueprints/Types/ResourceProgress` (`BlueprintMapLibrary.Map_Find` _requiredresource _array_element))))
  (`self.UpdateCollectedResource`)
  (`BoxComponent.SetBoxExtent` _boundbox (`self.GetBoundBoxSize` _buildingclass) true)
  (`SceneComponent.K2_SetRelativeLocation` _boundbox _returnvalue false false)
  (`SceneComponent.K2_SetRelativeLocation` (`self.Widget`) _returnvalue false false))

(event `self.BoundBox.OnComponentBeginOverlap`
  (params (OverlappedComponent :type "PrimitiveComponent Object Reference") (OtherActor :type "Actor Object Reference") (OtherComp :type "PrimitiveComponent Object Reference") (OtherBodyIndex :type Integer) (bFromSweep :type Boolean) (SweepResult :type "HitResult Structure (by ref)"))
  ;[1 1 1] OnOverlap
  (`self.UpdateCollectedResource` :!label _label))

(event `self.BoundBox.OnComponentEndOverlap`
  (params (OverlappedComponent :type "PrimitiveComponent Object Reference") (OtherActor :type "Actor Object Reference") (OtherComp :type "PrimitiveComponent Object Reference") (OtherBodyIndex :type Integer))
  ;[1 1 1] OnOverlap
  (goto _label))

(event `self.ReceiveTick`
  (params (DeltaSeconds :type "Float (single-precision)"))
  ;[1 1 1] Tick
  (if (`self.IsConstructing`)
    (`self.UpdateConstructionProgress` DeltaSeconds)
    (if (>= (`self.ConstructionProgress`) 1.0)
      (`self.FinishConstrtuction`))))

(event `FinishConstrtuction`
  ;[1 1 1] Finish Construction
  (`/Engine/EditorBlueprintResources/ActorMacros.Switch Has Authority`
    (:`Authority`
      (bind _keys (`BlueprintMapLibrary.Map_Keys` (`self.CollectedResources`)))
      (for _array_element _keys
        (`self.DestroyCollectedResource` _array_element))
      (`|SpawnActorFromClass` (`self.ConstructingBuildingClass`) (`self.GetTransform`) "Undefined" "MultiplyWithRoot" null null)
      (`self.K2_DestroyActor`))))

(fn `DestroyCollectedResource`
  (params (ResourceType :type "EResourceType Enum (by ref)"))
  (bind _objects (`self.GetAllOverlapingResourcesObjects` ResourceType))
  (for _index (range (`.RequiredAmount_2_E6F6DF9B4042BCDF0C96699D62E98C08` (break `/Game/Survival/Blueprints/Types/ResourceProgress` (`BlueprintMapLibrary.Map_Find` (`self.CollectedResources`) ResourceType))))
    (bind _asactor (cast `Actor` (`|GetArrayItem` _objects _index)))
    (`self.K2_DestroyActor` _asactor)))

(fn `GetAllOverlapingResourcesObjects`
  (params (ResourceType :type "EResourceType Enum" :default "Wood"))
  (returns (Objects :type "Array of Object Object Reference") (Size :type Integer))
  (locals (ResultArray :type "Array of Object Object Reference"))
  (`KismetArrayLibrary.Array_Clear` (`local.ResultArray`))
  (for _array_element (`self.GetOverlappingActors` null)
    (if (`self.IsAResource` _array_element ResourceType)
      (`KismetArrayLibrary.Array_Add` (`local.ResultArray`) _array_element)))
  (return (`local.ResultArray`) (`KismetArrayLibrary.Array_Length` (`local.ResultArray`))))

(fn `GetResourceTag`
  (params (Key :type "EResourceType Enum (by ref)"))
  (returns (Value :type "GameplayTag Structure"))
  (return (`BlueprintMapLibrary.Map_Find` (`/Game/Survival/Blueprints/Types/ResourceTagsDataAsset.ResourcesTags` (`self.ResourcesTags`)) Key)))

(fn `HasCollectedAllResources`
  (returns (`Collected AllResources` :type Boolean))
  (bind _values (`BlueprintMapLibrary.Map_Values` (`self.CollectedResources`)))
  (for _array_element _values
    (bind (_requiredamount _collectedamount) (break `/Game/Survival/Blueprints/Types/ResourceProgress` _array_element))
    (if (< _collectedamount _requiredamount)
      (return false)))
  (return true))

(fn `IsAResource`
  (params (Object :type "Object Object Reference") (ResourceTag :type "EResourceType Enum" :default "Wood"))
  (returns (Result :type Boolean))
  (bind _asitem (cast `Item` Object)
    (:`then`
      (bind _tagcontainer (message `GameplayTagAssetInterface.GetOwnedGameplayTags` _asitem))
      (return (`BlueprintGameplayTagLibrary.HasTag` _tagcontainer (`self.GetResourceTag` ResourceTag))))
    (:`CastFailed`
      (return false))))

(fn `OnRep_ConstructionProgress`
  (`/Engine/EditorBlueprintResources/ActorMacros.Switch Has Authority`
    (:`Remote`
      (bind _aswbp_construtciton (cast `/Game/Survival/Blueprints/Widgets/WBP_Construtciton` (`WidgetComponent.GetWidget` (`self.Widget`))))
      (`/Game/Survival/Blueprints/Widgets/WBP_Construtciton.SetProgress` _aswbp_construtciton (`self.ConstructionProgress`)))))

(fn `ResetCollectedAmount`
  (bind _keys (`BlueprintMapLibrary.Map_Keys` (`self.CollectedResources`)))
  (for _array_element _keys
    (`BlueprintMapLibrary.Map_Add` (`self.CollectedResources`) _array_element (make `/Game/Survival/Blueprints/Types/ResourceProgress` (`.RequiredAmount_2_E6F6DF9B4042BCDF0C96699D62E98C08` (break `/Game/Survival/Blueprints/Types/ResourceProgress` (`BlueprintMapLibrary.Map_Find` (`self.CollectedResources`) _array_element)))))))

(fn `SetBuildingClass`
  (params (ConstructingBuildingClass :type "Actor Class Reference"))
  (set `self.ConstructingBuildingClass` ConstructingBuildingClass))

(fn `SetCollectedResourceAmount`
  (params (ResourceType :type "EResourceType Enum (by ref)") (Amount :type Integer))
  (`BlueprintMapLibrary.Map_Add` (`self.CollectedResources`) ResourceType (make `/Game/Survival/Blueprints/Types/ResourceProgress` (`.RequiredAmount_2_E6F6DF9B4042BCDF0C96699D62E98C08` (break `/Game/Survival/Blueprints/Types/ResourceProgress` (`BlueprintMapLibrary.Map_Find` (`self.CollectedResources`) ResourceType))) Amount)))

(fn `StartConstructing`
  (`/Engine/EditorBlueprintResources/ActorMacros.Switch Has Authority`
    (:`Authority`
      (if (`self.HasCollectedAllResources`)
        (set `self.IsConstructing` true)
        (`self.SetActorTickEnabled` true)))))

(fn `StopConstructing`
  (set `self.IsConstructing` false)
  (`self.SetActorTickEnabled` false))

(fn `UpdateCollectedResource`
  (`self.ResetCollectedAmount`)
  (bind _keys (`BlueprintMapLibrary.Map_Keys` (`self.CollectedResources`)))
  (for _array_element _keys
    (bind (_objects _size) (`self.GetAllOverlapingResourcesObjects` _array_element))
    (`self.SetCollectedResourceAmount` _array_element _size))
  (`self.UpdateResourceWIdget`))

(fn `UpdateConstructionProgress`
  (params (DeltaTime :type "Float (double-precision)"))
  (bind _output_get (set `self.ConstructionProgress` (+ (* DeltaTime (`self.ConstructingSpeed`)) (`self.ConstructionProgress`))))
  (bind _aswbp_construtciton (cast `/Game/Survival/Blueprints/Widgets/WBP_Construtciton` (`WidgetComponent.GetWidget` (`self.Widget`))))
  (`/Game/Survival/Blueprints/Widgets/WBP_Construtciton.SetProgress` _aswbp_construtciton _output_get))

(fn `UpdateResourceWIdget`
  (bind _aswbp_construtciton (cast `/Game/Survival/Blueprints/Widgets/WBP_Construtciton` (`WidgetComponent.GetWidget` (`self.Widget`))))
  (`/Game/Survival/Blueprints/Widgets/WBP_Construtciton.Update` _aswbp_construtciton (`self.CollectedResources`)))

(fn `UserConstructionScript`)
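; BP_Pallete is a pallet game object that collects logs entering its effect area into its inventory.
; On overlap it binds to the log's state-change event and stores the log in the CarryingSocket.Log container if unattached.
; Items that later switch to the dropped state while unattached are added the same way.
; The actor's end-overlap event unbinds the state listener from departing items.
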(event `self.ReceiveBeginPlay`)

(event `self.Effect Area.OnComponentBeginOverlap`
  (params (OverlappedComponent :type "PrimitiveComponent Object Reference") (OtherActor :type "Actor Object Reference") (OtherComp :type "PrimitiveComponent Object Reference") (OtherBodyIndex :type Integer) (bFromSweep :type Boolean) (SweepResult :type "HitResult Structure (by ref)"))
  (bind _asbp_log (cast `/Game/Survival/Blueprints/Items/BP_Log` OtherActor))
  (add `Item.OnStateChanged` _asbp_log (delegate `CustomEvent`))
  (if (not (`Item.IsAttached` _asbp_log))
    (`InventoryComponent.AddItemToContainer` (`self.Inventory`) _asbp_log (struct :`TagName` "CarryingSocket.Log"))))

(event `CustomEvent`
  (params (Item :type "Actor Object Reference") (State :type "EItemStateChange Enum" :default "Drop"))
  (bind _asitem (cast `Item` Item))
  (if (not (`Item.IsAttached` _asitem))
    (if (`|EnumEquality` State "Droped")
      (`InventoryComponent.AddItemToContainer` (`self.Inventory`) _asitem (struct :`TagName` "CarryingSocket.Log")))))

(event `self.ReceiveActorEndOverlap`
  (params (OtherActor :type "Actor Object Reference"))
  (bind _asitem (cast `Item` OtherActor))
  (remove `Item.OnStateChanged` _asitem (delegate `CustomEvent`)))

(fn `UserConstructionScript`)
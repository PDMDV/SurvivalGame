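; Behavior tree service that finds the character nearest to the AI's controlled pawn and stores it as the target.
; On each tick it clears its actor list, then gathers all actors of every class in the CharacterClass array with GetAllActorsOfClass.
; FindNearestActor picks the closest one to the pawn's location, and the result is written to the TargetActor blackboard key.
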(event `self.ReceiveTickAI`
  (params (OwnerController :type "AIController Object Reference") (ControlledPawn :type "Pawn Object Reference") (DeltaSeconds :type "Float (single-precision)"))
  (`KismetArrayLibrary.Array_Clear` (`self.ActorsArray`))
  (for _array_element (`self.CharacterClass`)
    (bind _outactors (`GameplayStatics.GetAllActorsOfClass` _array_element))
    (`KismetArrayLibrary.Array_Append` (`self.ActorsArray`) _outactors))
  (`BTFunctionLibrary.SetBlackboardValueAsObject` (`self.TargetActor`) (`.ReturnValue` (`GameplayStatics.FindNearestActor` (`Actor.K2_GetActorLocation` ControlledPawn) (`self.ActorsArray`)))))
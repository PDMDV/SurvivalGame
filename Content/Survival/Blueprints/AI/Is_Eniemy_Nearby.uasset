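; Behavior tree decorator that checks whether any actor of the listed enemy classes is near the owning AI actor.
; PerformConditionCheck gets all actors of a class from EnemyType and passes on the first one closer to the owner than Distance.
; It returns false as soon as the first class yields no match, so later classes in the array are never checked.
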(fn `PerformConditionCheck`
  (params (OwnerActor :type "Actor Object Reference"))
  (returns (ReturnValue :type Boolean))
  (for _array_element (`self.EnemyType`)
    (bind _outactors (`GameplayStatics.GetAllActorsOfClass` _array_element))
    (for _array_element_2 _outactors
      (if (< (`KismetMathLibrary.Vector_Distance` (`Actor.K2_GetActorLocation` _array_element_2) (`Actor.K2_GetActorLocation` OwnerActor)) (`self.Distance`))
        (return true)))
    (return false)))
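; Gameplay ability for building placement, activated by an event carrying a BuildingDataAsset.
; The local client spawns a BP_PlacingBuilding preview that follows the mouse trace, optionally grid-snapped, and rotates in 90-degree steps on input.
; On valid placement, it sends the place event with the asset and a hit result packing location and facing into Normal.
; The cancel event destroys the BP_ConstructingBuilding under the cursor, using target data sent to the server.
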(event `self.K2_ActivateAbilityFromEvent`
  (params (EventData :type "GameplayEventData Structure (by ref)"))
  (bind _placingbuildingactor (`self.PlacingBuildingActor`))
  (bind _builidnglocation (`self.BuilidngLocation`))
  (bind _placingbuildingactor_2 (`self.PlacingBuildingActor`))
  (bind _placeabilitytag (`self.PlaceAbilityTag`))
  (bind _placingbuildingactor_3 (`self.PlacingBuildingActor`))
  ;[1 1 1] Init
  (bind _asbuilding_data_asset (cast `BuildingDataAsset` (`.OptionalObject` (break `GameplayEventData` EventData))))
  (set `self.BuildingAsset` _asbuilding_data_asset)
  (`self.IsLocallyControlled`
    (:`True`
      (bind _returnvalue (`|SpawnActorFromClass` "/Game/Survival/Blueprints/GameObjects/BP_PlacingBuilding.BP_PlacingBuilding_C" (`KismetMathLibrary.MakeTransform` (0.0 0.0 0.0)) "Undefined" "MultiplyWithRoot" null (`self.BuildingAsset`) null))
      (`/Engine/EditorBlueprintResources/StandardMacros.IsValid` _returnvalue
        (:`Is Valid`
          (set `self.PlacingBuildingActor` _returnvalue))))
    (:`False`
      _))
  (`|ExecutionSequence`
    (:`then_0`
      ;[1 1 1] Trace Mouse Position
      (`self.IsLocallyControlled`
        (:`True`
          (bind (_asynctaskproxy _data) (`AbilityTask_GetMouseHit.CreateGetMouseHit` "None" false false)
            (:`MouseDataReceived`
              (if (`BuildingDataAsset.SnapToGrid` (`self.BuildingAsset`))
                (bind _returnvalue_2 (+ (`.ImpactPoint` (`GameplayStatics.BreakHitResult` (`AbilitySystemBlueprintLibrary.GetHitResultFromTargetData` _data))) (0.0 0.0 1.0)))
                (set `self.BuilidngLocation` (`KismetMathLibrary.MakeVector` (`KismetMathLibrary.GridSnap_Float` (.x _returnvalue_2) 100.0) (`KismetMathLibrary.GridSnap_Float` (.y _returnvalue_2) 100.0) (.z _returnvalue_2)))
                (else
                  (set `self.BuilidngLocation` _returnvalue_2)))
              (`/Engine/EditorBlueprintResources/StandardMacros.IsValid` _placingbuildingactor
                (:`Is Valid`
                  (`Actor.K2_SetActorLocation` _placingbuildingactor (`self.BuilidngLocation`) true false))))))))
    (:`then_1`
      ;[1 1 1] Wait for placement
      (bind _asynctaskproxy_2 (`AbilityAsync_WaitGameplayEvent.WaitGameplayEventToActor` (`self.GetOwningActorFromActorInfo`) (`self.PlacementInputTag`))
        (:`then`
          (set `self.WaitToInputAsyncTask` _asynctaskproxy_2))
        (:`EventReceived`
          (`/Engine/EditorBlueprintResources/StandardMacros.IsValid` _placingbuildingactor_3
            (:`Is Valid`
              (if (`/Game/Survival/Blueprints/GameObjects/BP_PlacingBuilding.HasValidPosition` _placingbuildingactor_3)
                (`AbilitySystemBlueprintLibrary.SendGameplayEventToActor` (`self.GetOwningActorFromActorInfo`) _placeabilitytag (make `GameplayEventData` _placeabilitytag null null (`self.BuildingAsset`) null (struct) (struct) (struct) 0.0 (`AbilitySystemBlueprintLibrary.AbilityTargetDataFromHitResult` (`GameplayStatics.MakeHitResult` false false 0.0 0.0 _builidnglocation _builidnglocation (`KismetMathLibrary.Conv_RotatorToVector` (`Actor.K2_GetActorRotation` (`self.PlacingBuildingActor`)))))))))))))
    (:`then_2`
      ;[1 1 1] Cancel Construction
      (`AbilityAsync_WaitGameplayEvent.WaitGameplayEventToActor` (`self.GetOwningActorFromActorInfo`) (`self.CancelPlacement`)
        (:`EventReceived`
          (bind (_asynctaskproxy_3 _data_2) (`AbilityTask_GetMouseHit.CreateGetMouseHit` "None")
            (:`MouseDataReceived`
              (bind _asbp_constructing_building (cast `/Game/Survival/Blueprints/GameObjects/BP_ConstructingBuilding` (`.HitActor` (`GameplayStatics.BreakHitResult` (`AbilitySystemBlueprintLibrary.GetHitResultFromTargetData` _data_2)))))
              (`Actor.K2_DestroyActor` _asbp_constructing_building))))))
    (:`then_3`
      ;[1 1 1] Rotate Object
      (`self.IsLocallyControlled`
        (:`True`
          (bind _asynctaskproxy_4 (`AbilityAsync_WaitGameplayEvent.WaitGameplayEventToActor` (`self.GetOwningActorFromActorInfo`) (`self.RotateInputTag`))
            (:`then`
              (set `self.Async Action` _asynctaskproxy_4))
            (:`EventReceived`
              (`Actor.K2_SetActorRotation` _placingbuildingactor_2 (`KismetMathLibrary.ComposeRotators` (`Actor.K2_GetActorRotation` _placingbuildingactor_2) (struct :`Yaw` 90.0)) false))))))))

(event `self.K2_OnEndAbility`
  (params (bWasCancelled :type Boolean))
  (bind _async_action (`self.Async Action`))
  (bind _placingbuildingactor (`self.PlacingBuildingActor`))
  ;[1 1 1] Destroy Placing Building Actor
  (`/Engine/EditorBlueprintResources/StandardMacros.IsValid` _placingbuildingactor
    (:`Is Valid`
      (`Actor.K2_DestroyActor` _placingbuildingactor))
    (:`Is Not Valid`
      _))
  (`AbilityAsync.EndAction` (`self.WaitToInputAsyncTask`))
  (`/Engine/EditorBlueprintResources/StandardMacros.IsValid` _async_action
    (:`Is Valid`
      (`AbilityAsync.EndAction` _async_action))))
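; GA_Block is an event-triggered Gameplay Ability that lets a BaseCharacter block with the Weapon passed in the event payload.
; Activation plays a random montage matching the block tag while listening for attack hit events.
; Hits from an instigator within a frontal yaw cone commit the ability and, if that succeeds, apply BlockEffect to the blocker's ASC.
; The server ends the ability on the block finish event.
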(event `self.K2_ActivateAbilityFromEvent`
  (params (EventData :type "GameplayEventData Structure (by ref)"))
  (bind _returnvalue (`self.GetOwningActorFromActorInfo`))
  ;[1 1 1] Init
  (bind _asweapon (cast `Weapon` (`.OptionalObject` (break `GameplayEventData` EventData))))
  (set `self.Weapon` _asweapon)
  (bind _asbase_character (cast `BaseCharacter` (`self.GetOwningActorFromActorInfo`))
    (:`then`
      (set `self.Character` _asbase_character)
      (`|ExecutionSequence`
        (:`then_0`
          ;[1 1 1] Start Block Animation
          (`AbilityTask_PlayMontageAndWait.CreatePlayMontageAndWaitProxy` "None" (`MyGameLibrary.GetRandomMontageWithTag` (`self.Character`) (`self.BlockMonatageTag`))))
        (:`then_1`
          ;[1 1 1] Reaction to Hit
          (bind (_asynctaskproxy _payload) (`AbilityTask_WaitGameplayEvent.WaitGameplayEvent` (struct :`TagName` "Ability.Attack.Hit") null)
            (:`EventReceived`
              (if (< (`KismetMathLibrary.Abs` (.yaw (`KismetMathLibrary.NormalizedDeltaRotator` (`Actor.K2_GetActorRotation` _returnvalue) (`KismetMathLibrary.FindLookAtRotation` (`Actor.K2_GetActorLocation` _returnvalue) (`Actor.K2_GetActorLocation` (`.Instigator` (break `GameplayEventData` _payload))))))) 50.0)
                (bind _returnvalue_2 (`self.K2_CommitAbility`))
                (if _returnvalue_2
                  (`MyAbilitySystemBlueprintLibrary.ApplyEffectToASC` (`self.BlockEffect`) (`AbilitySystemBlueprintLibrary.GetAbilitySystemComponent` (`self.Character`))))))))
        (:`then_2`
          ;[1 1 1] Wait For Ability End
          (`self.K2_HasAuthority`
            (:`True`
              (`AbilityTask_WaitGameplayEvent.WaitGameplayEvent` (struct :`TagName` "Ability.Block.Finish") null
                (:`EventReceived`
                  (`self.K2_EndAbility`))))))))
    (:`CastFailed`
      (`self.K2_EndAbility`))))
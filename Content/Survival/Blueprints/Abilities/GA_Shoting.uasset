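; Gameplay ability for ranged shooting with an aimed, arrow-style weapon, moving the item from inventory slot to holding socket while active.
; Gameplay events toggle player aiming; firing while aiming plays the Shot montage and awaits its attack notify.
; The authority then spawns BP_Projectile at the Arrow_Slot socket, keeping only yaw.
; Overlapping an ASC owner applies weapon damage and destroys the projectile; blocking hits disable collision and set a short lifespan.
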(event `self.K2_ActivateAbilityFromEvent`
  (params (EventData :type "GameplayEventData Structure (by ref)"))
  ;[1 1 1] Init
  (set `self.Event Data` EventData)
  (bind _asbase_character (cast `BaseCharacter` (`self.GetOwningActorFromActorInfo`))
    (:`then`
      (bind _output_get (set `self.Character` _asbase_character))
      (bind _output_get_2 (set `self.Item` (`|GetArrayItem` (`InventoryComponent.GetItemsFromContainer` (`BaseCharacter.InventoryComponent` _output_get) (`self.InventorySlot`)))))
      (`Item.ApplyCarryingEffect` _output_get_2 (`self.Character`))
      (`InventoryComponent.SwitchItemContainer` (`BaseCharacter.InventoryComponent` (`self.Character`)) (`self.Item`) (`self.InventorySlot`) (`self.HoldingSocket`))
      (`|ExecutionSequence`
        (:`then_0`
          ;[1 1 1] Action1 Start - Start Aiming
          (`AbilityTask_WaitGameplayEvent.WaitGameplayEvent` (`self.Action2StartTag`) null
            (:`EventReceived`
              (set `self.bIsInputActionActive` true)
              (bind _asbp_player_character (cast `/Game/Survival/Blueprints/Characters/Player/BP_PlayerCharacter` (`self.Character`)))
              (`/Game/Survival/Blueprints/Characters/Player/BP_PlayerCharacter.SetIsAiming` _asbp_player_character true))))
        (:`then_1`
          ;[1 1 1] Action 1 End - Stop Aiming
          (`AbilityTask_WaitGameplayEvent.WaitGameplayEvent` (`self.Action2EndTag`) null
            (:`EventReceived`
              (set `self.bIsInputActionActive` false)
              (bind _asbp_player_character_2 (cast `/Game/Survival/Blueprints/Characters/Player/BP_PlayerCharacter` (`self.Character`)))
              (`/Game/Survival/Blueprints/Characters/Player/BP_PlayerCharacter.SetIsAiming` _asbp_player_character_2 false))))
        (:`then_2`
          ;[1 1 1] Action 2 Start - Shot
          (`AbilityTask_WaitGameplayEvent.WaitGameplayEvent` (`self.ActionStartTag`) null
            (:`EventReceived`
              (if (`self.bIsInputActionActive`)
                (`AbilityTask_PlayMontageAndWait.CreatePlayMontageAndWaitProxy` "None" "/Game/Survival/Anim/Archery/Shot.Shot"
                  (:`then`
                    (`AbilityTask_WaitGameplayEvent.WaitGameplayEvent` (struct :`TagName` "Anim.Notify.Atack") null true
                      (:`EventReceived`
                        (`self.K2_HasAuthority`
                          (:`True`
                            (bind _returnvalue (`|SpawnActorFromClass` "/Game/Survival/Blueprints/Items/BP_Projectile.BP_Projectile_C" (`KismetMathLibrary.MakeTransform` (.location (`SceneComponent.GetSocketTransform` (`StaticMeshActor.StaticMeshComponent` (`self.Item`)) "Arrow_Slot" "RTS_World")) (`KismetMathLibrary.MakeRotator` 0.0 0.0 (.yaw (.rotation (`SceneComponent.GetSocketTransform` (`StaticMeshActor.StaticMeshComponent` (`self.Item`)) "Arrow_Slot" "RTS_World")))) (.scale (`SceneComponent.GetSocketTransform` (`StaticMeshActor.StaticMeshComponent` (`self.Item`)) "Arrow_Slot" "RTS_World"))) "Undefined" "MultiplyWithRoot" null (`|MakeArray` (`self.Character`) (`self.Item`) :!type "Actor Object Reference") null))
                            (add `Actor.OnActorBeginOverlap` _returnvalue (delegate `Hit`))
                            (add `Actor.OnActorHit` _returnvalue (delegate `OnActorHit_Event`))))))))))))))
    (:`CastFailed`
      (`self.K2_EndAbility`))))

(event `self.K2_OnEndAbility`
  (params (bWasCancelled :type Boolean))
  ;[1 1 1] Ability End
  (bind _asbp_player_character (cast `/Game/Survival/Blueprints/Characters/Player/BP_PlayerCharacter` (`self.Character`)))
  (`/Game/Survival/Blueprints/Characters/Player/BP_PlayerCharacter.SetIsAiming` _asbp_player_character false)
  (`Item.RemoveCarryingEffect` (`self.Item`) (`self.Character`))
  (`InventoryComponent.SwitchItemContainer` (`BaseCharacter.InventoryComponent` (`self.Character`)) (`self.Item`) (`self.HoldingSocket`) (`self.InventorySlot`)))

(event `OnActorHit_Event`
  (params (SelfActor :type "Actor Object Reference") (OtherActor :type "Actor Object Reference") (NormalImpulse :type "Vector Structure") (Hit :type "HitResult Structure (by ref)"))
  ;[1 1 1] Hit
  (`Actor.SetActorEnableCollision` SelfActor false)
  (`Actor.SetLifeSpan` SelfActor 3.0))

(event `Hit`
  (params (OverlappedActor :type "Actor Object Reference") (OtherActor :type "Actor Object Reference"))
  (bind _returnvalue (`AbilitySystemBlueprintLibrary.GetAbilitySystemComponent` OtherActor))
  ;[1 1 1] Character Hit
  (bind _asweapon (cast `Weapon` (`self.Item`)))
  (if (`KismetSystemLibrary.IsValid` _returnvalue)
    (`MyAbilitySystemBlueprintLibrary.ApplyEffectToASC` (`Weapon.GetDamageEffect` _asweapon) _returnvalue)
    (`Actor.K2_DestroyActor` OverlappedActor)))

(fn `SetOptionalObjectAndGameplayTag`
  (params (InGameplayEvent :type "GameplayEventData Structure") (`Optional Object` :type "Object Object Reference") (`Event Tag` :type "GameplayTag Structure"))
  (returns (GameplayEventData :type "GameplayEventData Structure"))
  (bind ((`Instigator` _instigator) (`Target` _target) (`OptionalObject2` _optionalobject2) (`ContextHandle` _contexthandle) (`InstigatorTags` _instigatortags) (`TargetTags` _targettags) (`EventMagnitude` _eventmagnitude) (`TargetData` _targetdata)) (break `GameplayEventData` InGameplayEvent))
  (return (make `GameplayEventData` `Event Tag` _instigator _target `Optional Object` _optionalobject2 _contexthandle _instigatortags _targettags _eventmagnitude _targetdata)))
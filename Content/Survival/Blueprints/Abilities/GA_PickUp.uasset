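; Gameplay ability that lets a character pick up an item, activated by a gameplay event carrying the item as Target and the character as Instigator.
; On authority only, it checks that the character's inventory can take the item, then applies the item's pick-up effect.
; If that succeeds, it removes the item from any inventory holding it and adds it to each matching container tag on the character's inventory.
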(event `self.K2_ActivateAbilityFromEvent`
  (params (EventData :type "GameplayEventData Structure (by ref)"))
  (bind (_eventtag _instigator _target) (break `GameplayEventData` EventData))
  (bind _hititem (`self.HitItem`))
  (bind _returnvalue (`InventoryComponent.GetItemInventory` (`self.HitItem`)))
  (bind _inventorycomponent (`BaseCharacter.InventoryComponent` (`self.LiftingCharacter`)))
  ;[1 1 1] PickUp
  (`self.K2_HasAuthority`
    (:`True`
      (bind _asitem (cast `Item` _target)
        (:`then`
          (set `self.HitItem` _asitem)
          (bind _asbase_character (cast `BaseCharacter` _instigator)
            (:`then`
              (set `self.LiftingCharacter` _asbase_character)
              (if (`InventoryComponent.CanPickUpItem` _inventorycomponent _hititem)
                (bind _returnvalue_2 (`Item.ApplyPickUpEffect` (`self.HitItem`) (`self.LiftingCharacter`)))
                (if _returnvalue_2
                  (`/Engine/EditorBlueprintResources/StandardMacros.IsValid` _returnvalue
                    (:`Is Valid`
                      (`InventoryComponent.RemoveItem` _returnvalue (`self.HitItem`)))
                    (:`Is Not Valid`
                      _))
                  (for _array_element (`BlueprintGameplayTagLibrary.BreakGameplayTagContainer` (`InventoryComponent.GetContainersForItem` _inventorycomponent _hititem))
                    (`InventoryComponent.AddItemToContainer` (`BaseCharacter.InventoryComponent` (`self.LiftingCharacter`)) (`self.HitItem`) _array_element))
                  (`self.K2_EndAbility`)
                  (else
                    (`self.K2_EndAbility` :!label _label)))
                (else
                  (goto _label))))
            (:`CastFailed`
              (`self.K2_EndAbility` :!label _label_2))))
        (:`CastFailed`
          (goto _label_2))))
    (:`False`
      (`self.K2_EndAbility`))))
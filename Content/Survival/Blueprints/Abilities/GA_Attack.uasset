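; Gameplay ability for a character's weapon attack, triggered by an event that carries the Weapon as its optional object.
; After committing, it plays a random tagged montage and ends when that stops or a finish event arrives, then sends an ended event.
; On the authority, the attack anim notify applies hit events and effects to ability-system targets in the weapon's area, or plain damage to GameObjects, then re-commits, ending on failure.
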(event `self.K2_ActivateAbilityFromEvent`
  (params (EventData :type "GameplayEventData Structure (by ref)"))
  ;[1 1 1] Init
  (bind _output_get (set `self.Event Data` EventData))
  (bind _asweapon (cast `Weapon` (`.OptionalObject` (break `GameplayEventData` _output_get)))
    (:`then`
      (set `self.Weapon` _asweapon)
      (bind _asbase_character (cast `BaseCharacter` (`self.GetOwningActorFromActorInfo`))
        (:`then`
          (set `self.Character` _asbase_character)
          (bind _returnvalue (`self.K2_CommitAbility`))
          (if _returnvalue
            (`|ExecutionSequence`
              (:`then_0`
                ;[1 1 1] Attack Animation
                (`AbilityTask_PlayMontageAndWait.CreatePlayMontageAndWaitProxy` "None" (`MyGameLibrary.GetRandomMontageWithTag` (`self.Character`) (`self.AttackMonatageTag`))
                  (:`OnCompleted`
                    _)
                  (:`OnInterrupted`
                    _)
                  (:`OnCancelled`
                    _))
                (`self.K2_EndAbility`))
              (:`then_1`
                ;[1 1 1] Apply Damage
                (`self.K2_HasAuthority`
                  (:`True`
                    (`AbilityTask_WaitGameplayEvent.WaitGameplayEvent` (struct :`TagName` "Anim.Notify.Atack") null
                      (:`EventReceived`
                        (`self.ApplyDamage`)
                        (bind _returnvalue_2 (`self.K2_CommitAbility`))
                        (if (not _returnvalue_2)
                          (`self.K2_EndAbility`)))))))
              (:`then_2`
                ;[1 1 1] Finish Ability
                (`AbilityTask_WaitGameplayEvent.WaitGameplayEvent` (struct :`TagName` "Ability.Attack.Finish") null
                  (:`EventReceived`
                    (`self.K2_EndAbility`)))))
            (else
              (`self.K2_EndAbility`))))
        (:`CastFailed`
          (`self.K2_EndAbility`))))
    (:`CastFailed`
      (`self.K2_EndAbility`))))

(event `self.K2_OnEndAbility`
  (params (bWasCancelled :type Boolean))
  ;[1 1 1] End Ability
  (`self.SendGameplayEvent` (struct :`TagName` "Ability.Attack.Ended")))

(fn `ApplyDamage`
  (bind _attackhittag (`self.AttackHitTag`))
  ;[1 1 1] Apply Damage
  (for _array_element (`Weapon.GetObjectsInDamageArea` (`self.Weapon`) null)
    (bind _returnvalue (`AbilitySystemBlueprintLibrary.GetAbilitySystemComponent` _array_element))
    (if (and (`KismetSystemLibrary.IsValid` _returnvalue) (!= _array_element (`self.Character`)))
      (`AbilitySystemBlueprintLibrary.SendGameplayEventToActor` _array_element _attackhittag (make `GameplayEventData` _attackhittag (`self.Character`) null (`self.Weapon`)))
      (`MyAbilitySystemBlueprintLibrary.ApplyEffectToASC` (`Weapon.GetDamageEffect` (`self.Weapon`)) _returnvalue)
      (`MyAbilitySystemBlueprintLibrary.ApplyEffectToASC` "/Game/Survival/Blueprints/Effects/GAE_RemoveHitBlockEffect.GAE_RemoveHitBlockEffect_C" _returnvalue)
      (else
        (bind _asgame_object (cast `GameObject` _array_element))
        (`GameplayStatics.ApplyDamage` _asgame_object (`self.BaseDamage`))))))
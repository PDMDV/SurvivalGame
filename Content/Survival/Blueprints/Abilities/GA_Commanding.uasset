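; GA_Commanding is a gameplay ability that shows the commanding abilities panel on the local player's HUD while it is active.
; On event-triggered activation it creates a WBP_AbilitiesPanel fed by the DA_Commanding_Abilities_Panel data asset.
; It reaches WBP_Overlay through the owning character's controller and MyHUD, then adds the panel to BottomSlot.
; Ending the ability removes the panel, with both UI steps limited to locally controlled instances.
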(event `self.K2_ActivateAbilityFromEvent`
  (params (EventData :type "GameplayEventData Structure (by ref)"))
  ;[1 1 1] Create UI
  (`self.IsLocallyControlled`
    (:`True`
      (`self.CreateBuildingWidget`))))

(event `self.K2_OnEndAbility`
  (params (bWasCancelled :type Boolean))
  ;[1 1 1] Destroy UI
  (`self.IsLocallyControlled`
    (:`True`
      (`Widget.RemoveFromParent` (`self.CommandingPanel`)))))

(fn `CreateBuildingWidget`
  ;[1 1 1] Create Building Widget
  (`self.IsLocallyControlled`
    (:`True`
      (bind _returnvalue (`|CreateWidget` "/Game/Survival/Blueprints/Widgets/WBP_AbilitiesPanel.WBP_AbilitiesPanel_C" null (struct) "/Game/Survival/Blueprints/DataAssets/UI/DA_Commanding_Abilities_Panel.DA_Commanding_Abilities_Panel"))
      (set `self.CommandingPanel` _returnvalue)
      (bind _hudoverlay (`self.GetHUDOverlay`))
      (`/Engine/EditorBlueprintResources/StandardMacros.IsValid` _hudoverlay
        (:`Is Valid`
          (`PanelWidget.AddChild` (`/Game/Survival/Blueprints/Widgets/WBP_Overlay.BottomSlot` _hudoverlay) (`self.CommandingPanel`)))))))

(fn `GetHUDOverlay`
  (returns (HUDOverlay :type "/Game/Survival/Blueprints/Widgets/WBP_Overlay Object Reference"))
  ;[1 1 1] GetHUDOverlay
  (bind _ascharacter (cast `Character` (`self.GetOwningActorFromActorInfo`)))
  (bind _asplayer_controller (cast `PlayerController` (`Pawn.GetController` _ascharacter)))
  (bind _asmy_hud (cast `MyHUD` (`PlayerController.GetHUD` _asplayer_controller)))
  (bind _aswbp_overlay (cast `/Game/Survival/Blueprints/Widgets/WBP_Overlay` (`MyHUD.GetOverlay` _asmy_hud)))
  (return _aswbp_overlay))
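; GA_PlaceBuilding is a gameplay ability that places a new construction site for a building, triggered by a gameplay event.
; On the server, it reads the BuildingDataAsset from the event's optional object and spawns BP_ConstructingBuilding at the target data's hit location, passing that asset along.
; The spawned actor's X axis follows the hit normal, and clients simply end the ability.
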(event `self.K2_ActivateAbilityFromEvent`
  (params (EventData :type "GameplayEventData Structure (by ref)"))
  (bind (_eventtag _instigator _target _optionalobject _optionalobject2 _contexthandle _instigatortags _targettags _eventmagnitude _targetdata) (break `GameplayEventData` EventData))
  (bind (_bblockinghit _binitialoverlap _time _distance _location _impactpoint _normal) (`GameplayStatics.BreakHitResult` (`AbilitySystemBlueprintLibrary.GetHitResultFromTargetData` _targetdata)))
  ;[1 1 1] Place Building
  (`self.K2_HasAuthority`
    (:`True`
      (bind _asbuilding_data_asset (cast `BuildingDataAsset` _optionalobject))
      (set `self.BuildingAsset` _asbuilding_data_asset)
      (`|SpawnActorFromClass` "/Game/Survival/Blueprints/GameObjects/BP_ConstructingBuilding.BP_ConstructingBuilding_C" (`KismetMathLibrary.MakeTransform` _location (`KismetMathLibrary.MakeRotFromX` _normal)) "Undefined" "MultiplyWithRoot" null (`self.BuildingAsset`) null)
      (`self.K2_EndAbility`))
    (:`False`
      (`self.K2_EndAbility`))))
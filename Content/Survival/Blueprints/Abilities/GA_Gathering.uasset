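; Gathering gameplay ability that relays a pickup request for the actor under the mouse.
; Once activated, it waits for the action-start event, then runs a GetMouseHit task that sends target data to the server.
; If the hit actor is within a short radius, it sends the owner a pickup gameplay event carrying both actors and their tags.
; On ability end, it drops the first item from each configured drop container in the character's inventory.
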(event `self.K2_ActivateAbilityFromEvent`
  (params (EventData :type "GameplayEventData Structure (by ref)"))
  (bind _pickupabilitytag (`self.PickUpAbilityTag`))
  ;[1 1 1] Gathering
  (`AbilityTask_WaitGameplayEvent.WaitGameplayEvent` (`self.ActionStartTag`) null
    (:`EventReceived`
      (bind (_asynctaskproxy _data) (`AbilityTask_GetMouseHit.CreateGetMouseHit` "None")
        (:`MouseDataReceived`
          (bind _tagcontainer (message `GameplayTagAssetInterface.GetOwnedGameplayTags` (`self.GetOwningActorFromActorInfo`)))
          (bind (_bblockinghit _binitialoverlap _time _distance _location _impactpoint _normal _impactnormal _physmat _hitactor) (`GameplayStatics.BreakHitResult` (`AbilitySystemBlueprintLibrary.GetHitResultFromTargetData` _data)))
          (bind _tagcontainer_2 (message `GameplayTagAssetInterface.GetOwnedGameplayTags` _hitactor))
          (if (`MyGameLibrary.IsInRadius` (`self.GetOwningActorFromActorInfo`) _hitactor 150.0)
            (`AbilitySystemBlueprintLibrary.SendGameplayEventToActor` (`self.GetOwningActorFromActorInfo`) _pickupabilitytag (make `GameplayEventData` _pickupabilitytag (`self.GetOwningActorFromActorInfo`) _hitactor null null (struct) _tagcontainer _tagcontainer_2))))))))

(event `self.K2_OnEndAbility`
  (params (bWasCancelled :type Boolean))
  ;[1 1 1] On End Ability Drop Carrying Items
  (bind _asbase_character (cast `BaseCharacter` (`self.GetOwningActorFromActorInfo`)))
  (for _array_element (`BlueprintGameplayTagLibrary.BreakGameplayTagContainer` (`self.DropContainers`))
    (bind _inventorycomponent (`BaseCharacter.InventoryComponent` _asbase_character))
    (`InventoryComponent.DropItem` _inventorycomponent (`InventoryComponent.GetFirstItemFromContainer` _inventorycomponent _array_element))))
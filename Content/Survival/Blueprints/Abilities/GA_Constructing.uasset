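; Gameplay ability that lets a character start and stop work on a construction site, triggered by an event carrying the tool.
; On the action-start event, a mouse-hit task sends target data, and the server starts constructing the hit BP_ConstructingBuilding if within Range.
; The action-end event stops construction on the server and clears the reference.
; An ApplyDamage helper for the tool's damage area is defined but not called here.
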(event `self.K2_ActivateAbilityFromEvent`
  (params (EventData :type "GameplayEventData Structure (by ref)"))
  (bind _constructingbuilding (`self.ConstructingBuilding`))
  ;[1 1 1] Init
  (bind _output_get (set `self.Event Data` EventData))
  (bind _asweapon (cast `Weapon` (`.OptionalObject` (break `GameplayEventData` _output_get)))
    (:`then`
      _)
    (:`CastFailed`
      _))
  (set `self.Tool` _asweapon)
  (bind _asbase_character (cast `BaseCharacter` (`self.GetOwningActorFromActorInfo`))
    (:`then`
      (set `self.Character` _asbase_character)
      (`|ExecutionSequence`
        (:`then_0`
          ;[1 1 1] Wait for Action Start
          (`AbilityTask_WaitGameplayEvent.WaitGameplayEvent` (`self.ActionStartTag`) null
            (:`EventReceived`
              (bind (_asynctaskproxy _data) (`AbilityTask_GetMouseHit.CreateGetMouseHit` "None")
                (:`MouseDataReceived`
                  (`self.K2_HasAuthority`
                    (:`True`
                      (bind _asbp_constructing_building (cast `/Game/Survival/Blueprints/GameObjects/BP_ConstructingBuilding` (`.HitActor` (`GameplayStatics.BreakHitResult` (`AbilitySystemBlueprintLibrary.GetHitResultFromTargetData` _data)))))
                      (if (`self.IsInRange` _asbp_constructing_building)
                        (bind _output_get_2 (set `self.ConstructingBuilding` _asbp_constructing_building))
                        (`/Game/Survival/Blueprints/GameObjects/BP_ConstructingBuilding.StartConstructing` _output_get_2)))))))))
        (:`then_1`
          ;[1 1 1] Wait for Action End
          (`AbilityTask_WaitGameplayEvent.WaitGameplayEvent` (`self.ActionEndTag`) null
            (:`EventReceived`
              (`self.K2_HasAuthority`
                (:`True`
                  (`/Engine/EditorBlueprintResources/StandardMacros.IsValid` _constructingbuilding
                    (:`Is Valid`
                      (`/Game/Survival/Blueprints/GameObjects/BP_ConstructingBuilding.StopConstructing` _constructingbuilding)
                      ;;[1 1 1] Set Null
                      (set `self.ConstructingBuilding` null))))))))))
    (:`CastFailed`
      (`self.K2_EndAbility`))))

(fn `ApplyDamage`
  (bind _tool (`self.Tool`))
  (`Weapon.DrawDebugDamageArea` _tool)
  (for _array_element (`Weapon.GetObjectsInDamageArea` _tool null)
    (bind _returnvalue (`AbilitySystemBlueprintLibrary.GetAbilitySystemComponent` _array_element))
    (if (and (`KismetSystemLibrary.IsValid` _returnvalue) (!= _array_element (`self.Character`)))
      (`AbilitySystemBlueprintLibrary.SendGameplayEventToActor` _array_element (struct) (make `GameplayEventData` (struct) (`self.Character`) null (`self.Tool`)))
      (`MyAbilitySystemBlueprintLibrary.ApplyEffectToASC` (`Weapon.GetDamageEffect` (`self.Tool`)) _returnvalue)
      (else
        (bind _asgame_object (cast `GameObject` _array_element))
        (`GameplayStatics.ApplyDamage` _asgame_object)))))

(fn `IsInRange`
  (params (self2 :type "Actor Object Reference"))
  (returns (ReturnValue :type Boolean))
  (return (< (`Actor.GetDistanceTo` self2 (`self.GetOwningActorFromActorInfo`)) (`self.Range`))))
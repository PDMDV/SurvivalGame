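; Gameplay ability for combat stance that moves the first item from an inventory slot to a holding socket and applies its carrying effect.
; Listens for input gameplay events and forwards them as attack and block events, passing the item as payload when starting either.
; Player-controlled characters repeat attacks while input stays active.
; When the ability ends, the authority removes the carrying effect and returns the item to its slot.
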(event `self.K2_ActivateAbilityFromEvent`
  (params (EventData :type "GameplayEventData Structure (by ref)"))
  (bind _blockabilitytag (`self.BlockAbilityTag`))
  (bind (_eventtag _instigator _target _optionalobject _optionalobject2 _contexthandle _instigatortags _targettags _eventmagnitude _targetdata) (break `GameplayEventData` (`self.Event Data`)))
  (bind _output (`|GetArrayItem` (`InventoryComponent.GetItemsFromContainer` (`BaseCharacter.InventoryComponent` (`self.Character`)) (`self.InventorySlot`))))
  ;[1 1 1] Init
  (set `self.Event Data` EventData)
  (bind _asbase_character (cast `BaseCharacter` (`self.GetOwningActorFromActorInfo`))
    (:`then`
      (set `self.Character` _asbase_character)
      (set `self.bEnableAutoAttack` (`Controller.IsPlayerController` (`Pawn.GetController` _asbase_character)))
      (`/Engine/EditorBlueprintResources/StandardMacros.IsValid` _output
        (:`Is Valid`
          (bind _output_get (set `self.Item` _output))
          (`Item.ApplyCarryingEffect` _output_get (`self.Character`))
          (`InventoryComponent.SwitchItemContainer` (`BaseCharacter.InventoryComponent` (`self.Character`)) (`self.Item`) (`self.InventorySlot`) (`self.HoldingSocket`))
          (`|ExecutionSequence`
            (:`then_0`
              ;[1 1 1] Action1 Start - Attack
              (`AbilityTask_WaitGameplayEvent.WaitGameplayEvent` (`self.ActionStartTag`) null
                (:`EventReceived`
                  (set `self.bIsInputActionActive` true)
                  (`self.Attack`))))
            (:`then_1`
              ;[1 1 1] Continue Attack if input is active
              (`AbilityTask_WaitGameplayEvent.WaitGameplayEvent` (`self.AttackEndedTag`) null
                (:`EventReceived`
                  (if (and (`self.bIsInputActionActive`) (`self.bEnableAutoAttack`))
                    (`self.Attack`)))))
            (:`then_2`
              ;[1 1 1] Action 1 End - End Attack
              (`AbilityTask_WaitGameplayEvent.WaitGameplayEvent` (`self.ActionEndTag`) null
                (:`EventReceived`
                  (set `self.bIsInputActionActive` false)
                  (`AbilitySystemBlueprintLibrary.SendGameplayEventToActor` (`self.GetOwningActorFromActorInfo`) (`self.FinishAttackTag`)))))
            (:`then_3`
              ;[1 1 1] Action 2 - Block
              (`AbilityTask_WaitGameplayEvent.WaitGameplayEvent` (`self.Action2Tag`) null
                (:`EventReceived`
                  (set `self.bIsBlocking` true)
                  (`AbilitySystemBlueprintLibrary.SendGameplayEventToActor` (`self.GetOwningActorFromActorInfo`) _blockabilitytag (make `GameplayEventData` _blockabilitytag _instigator _target (`self.Item`) _optionalobject2 _contexthandle _instigatortags _targettags _eventmagnitude _targetdata)))))
            (:`then_4`
              ;[1 1 1] Action 2 End - Block End
              (`AbilityTask_WaitGameplayEvent.WaitGameplayEvent` (`self.Action2EndTag`) null
                (:`EventReceived`
                  (set `self.bIsInputAction2Active` false)
                  (`AbilitySystemBlueprintLibrary.SendGameplayEventToActor` (`self.GetOwningActorFromActorInfo`) (struct :`TagName` "Ability.Block.Finish"))
                  (set `self.bIsBlocking` false))))))
        (:`Is Not Valid`
          (`self.K2_EndAbility`))))
    (:`CastFailed`
      (`self.K2_EndAbility`))))

(event `self.K2_OnEndAbility`
  (params (bWasCancelled :type Boolean))
  ;[1 1 1] OnAbilityEnd
  (`self.K2_HasAuthority`
    (:`True`
      (`Item.RemoveCarryingEffect` (`self.Item`) (`self.Character`))
      (`InventoryComponent.SwitchItemContainer` (`BaseCharacter.InventoryComponent` (`self.Character`)) (`self.Item`) (`self.HoldingSocket`) (`self.InventorySlot`)))))

(fn `Attack`
  (bind _attackabilitytag (`self.AttackAbilityTag`))
  (`AbilitySystemBlueprintLibrary.SendGameplayEventToActor` (`self.GetOwningActorFromActorInfo`) _attackabilitytag (`self.SetOptionalObjectAndGameplayTag` (`self.Event Data`) (`self.Item`) _attackabilitytag)))

(fn `SetOptionalObjectAndGameplayTag`
  (params (InGameplayEvent :type "GameplayEventData Structure") (`Optional Object` :type "Object Object Reference") (`Event Tag` :type "GameplayTag Structure"))
  (returns (GameplayEventData :type "GameplayEventData Structure"))
  (bind ((`Instigator` _instigator) (`Target` _target) (`OptionalObject2` _optionalobject2) (`ContextHandle` _contexthandle) (`InstigatorTags` _instigatortags) (`TargetTags` _targettags) (`EventMagnitude` _eventmagnitude) (`TargetData` _targetdata)) (break `GameplayEventData` InGameplayEvent))
  (return (make `GameplayEventData` `Event Tag` _instigator _target `Optional Object` _optionalobject2 _contexthandle _instigatortags _targettags _eventmagnitude _targetdata)))
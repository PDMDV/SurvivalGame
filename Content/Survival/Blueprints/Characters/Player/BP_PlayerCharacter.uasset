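; Player character Blueprint for a survival game that gives the player a wolf companion and relays aiming state to animation.
; After a short delay from BeginPlay, SpawnCompanion runs on authority only, spawning BP_Wolf at a random navigable point near the player and storing it as Companion.
; The SetIsAiming event casts the mesh's anim instance to BP_PlayerAnim and sets its IsAiming flag.
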(event `self.ReceiveBeginPlay`
  (`KismetSystemLibrary.Delay` 10.0)
  (`self.SpawnCompanion`))

(event `self.ReceiveTick`
  (params (DeltaSeconds :type "Float (single-precision)")))

(event `SetIsAiming`
  (params (IsAiming :type Boolean))
  (bind _asbp_player_anim (cast `/Game/Survival/Anim/BP_PlayerAnim` (`SkeletalMeshComponent.GetAnimInstance` (`self.Mesh`))))
  (set `/Game/Survival/Anim/BP_PlayerAnim.bIsAiming` IsAiming _asbp_player_anim))

(fn `SpawnCompanion`
  (`/Engine/EditorBlueprintResources/ActorMacros.Switch Has Authority`
    (:`Authority`
      (bind _randomlocation (`NavigationSystemV1.K2_GetRandomLocationInNavigableRadius` (`self.K2_GetActorLocation`) 300.0 null null))
      (bind _returnvalue (`|SpawnActorFromClass` "/Game/Survival/Blueprints/Characters/Enemies/Wolf/BP_Wolf.BP_Wolf_C" (`KismetMathLibrary.MakeTransform` _randomlocation) "Undefined" "MultiplyWithRoot" null null))
      (set `self.Companion` _returnvalue))))

(fn `UserConstructionScript`)
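; Custom PCG element that turns the terrain map of the owning BP_Terrain actor into points for the requested terrain types.
; It reads the terrain type array and actor location, then runs an iteration loop over every cell.
; Each cell maps to a cell-centered point on a 50-wide, 100-unit grid, seeded by position.
; Only points whose type is in RequestedTypes are kept.
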(fn ExecutewithContext
  (params (InContext :type PCG%20Context%20Structure%20%28by%20ref%29) (Input :type PCG%20Data%20Collection%20Structure%20%28by%20ref%29))
  (bind _output_get (LocalVariables|SetContext InContext))
  (bind _returnvalue (PCG|Temporary|GetComponent _output_get))
  (bind _asbp_terrain (Utilities|Casting|CastToBP_Terrain (Components|GetOwner _returnvalue)))
  (bind _output_get_2 (Variables|Default|SetTerrainMap (Class|Terrain|GetTerrainTypeArray _asbp_terrain)))
  (Variables|Default|SetLocation (Transformation|GetActorLocation _asbp_terrain))
  (bind _outdata (PCG|FlowControl|IterationLoop (LocalVariables|GetContext) (Class|KismetMathLibrary|ToInt64(Integer) (Utilities|Array|Length _output_get_2)) 0 0 0))
  (return (Utilities|Struct|MakePCGDataCollection (Utilities|Array|MakeArray (Utilities|Struct|MakePCGTaggedData _outdata 0 "None")))))

(fn IterationLoopBody
  (params (InContext :type PCG%20Context%20Structure%20%28by%20ref%29) (Iteration :type Integer64) (InA :type PCG%20Spatial%20Data%20Object%20Reference) (InB :type PCG%20Spatial%20Data%20Object%20Reference) (OutMetadata :type PCG%20Metadata%20Object%20Reference))
  (bind _returnvalue (Class|KismetMathLibrary|PercentInt64Int64 Iteration 50))
  (bind _returnvalue_2 (/ Iteration 50))
  (bind _location (Variables|Default|GetLocation))
  (bind _returnvalue_3 (* _returnvalue 100))
  (bind _returnvalue_4 (* _returnvalue_2 100))
  (bind _returnvalue_5 (Math|Conversions|ToFloat(Integer) _returnvalue_3))
  (bind _returnvalue_6 (Math|Conversions|ToFloat(Integer) _returnvalue_4))
  (bind _returnvalue_7 (Math|Vector|MakeVector _returnvalue_5 _returnvalue_6 1e+02))
  (bind _returnvalue_8 (+ _returnvalue_7 "50.000000,50.000000,-100.000000" _location))
  (bind _returnvalue_9 (PCG|Helpers|ComputeSeedfromPosition _returnvalue_8))
  (return (Utilities|Struct|MakePCGPoint (Math|Transform|MakeTransform _returnvalue_8) "-45.000000,-45.000000,-10.000000" "45.000000,45.000000,10.000000" _returnvalue_9) (Utilities|Set|Contains (Variables|Default|GetRequestedTypes) (Utilities|Array|Get(acopy) (Variables|Default|GetTerrainMap) (Math|Conversions|ToInteger(Byte) Iteration)))))